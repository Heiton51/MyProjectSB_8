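; Player pawn that slides sideways along the Y axis and spawns the ball it plays with.
; MoveRight input applies a fixed, swept world offset each call in either direction, with no delta-time scaling.
; BeginPlay calls SpawnBall, which creates a BP_Ball at the capsule's transform and stores it as PlayingBall.
; It then binds the ball's OnDead event to OnDeadReaction, which is currently empty.
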(event `InputAxis|MoveRight`
  (params (AxisValue :type "Float (single-precision)"))
  (if (< AxisValue 0.0)
    (`self.K2_AddActorWorldOffset` (0.0 -75.0 0.0) true)))

(event `InputAxis|MoveRight`
  (params (AxisValue :type "Float (single-precision)"))
  (if (> AxisValue 0.0)
    (`self.K2_AddActorWorldOffset` (0.0 75.0 0.0) true)))

(event `self.ReceiveBeginPlay`
  (bind _output_get (`self.SpawnBall`))
  (add `/Game/BP_Ball.OnDead` _output_get (delegate `OnDeadReaction`)))

(event `OnDeadReaction`)

(event `self.ReceiveTick`
  (params (DeltaSeconds :type "Float (single-precision)")))

(fn `SpawnBall`
  (returns (Output_Get :type "/Game/BP_Ball Object Reference"))
  (bind _returnvalue (`|SpawnActorFromClass` "/Game/BP_Ball.BP_Ball_C" (`SceneComponent.K2_GetComponentToWorld` (`self.Capsule`)) "AlwaysSpawn" "OverrideRootScale" null null))
  (set `self.PlayingBall` _returnvalue))

(fn `UserConstructionScript`)